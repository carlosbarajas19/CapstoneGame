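; BP_DemoScene is a scene setup actor for the StylizedShields demo, configuring lighting and a cube from exposed variables.
; Its construction script rotates the directional light as the sun and sets the cube's visibility, location and scale.
; It then offsets the skylight vertically by a height variable and recaptures the sky.
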(fn ConstructionScript
  (Transformation|SetWorldRotation (Variables|Default|GetDirectionalLight) (Variables|Default|GetRotSun) false false)
  (Rendering|SetVisibility (Variables|Default|GetCube) (Variables|Default|GetCubeVisible) false)
  (Transformation|SetRelativeTransform (Variables|Default|GetCube) (Math|Transform|MakeTransform (Variables|Default|GetLocCube) "0, 0, 0" (Variables|Default|GetScaleCube)) false false)
  (Transformation|AddLocalOffset (Variables|Default|GetSkyLight) (Math|Vector|MakeVector 0.0 0.0 (Variables|Default|GetSkyLightHeight)) false false)
  (Class|SkyLightComponent|RecaptureSky (Variables|Default|GetSkyLight)))