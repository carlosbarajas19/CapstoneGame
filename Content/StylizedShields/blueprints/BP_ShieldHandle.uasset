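; BP_ShieldHandle is a Blueprint in the StylizedShields pack that assembles a shield with its handle from two static mesh components.
; Its construction script assigns the mesh and slot-zero material of the Handle and Shield components from separate variables, so each part's look is configurable.
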(fn ConstructionScript
  (Components|StaticMesh|SetStaticMesh (Variables|Default|Gethandle) (Variables|Default|GetSM_handle))
  (Rendering|Material|SetMaterial (Variables|Default|Gethandle) 0 (Variables|Default|GetM_handle))
  (Components|StaticMesh|SetStaticMesh (Variables|Default|Getshield) (Variables|Default|GetSM_shield))
  (Rendering|Material|SetMaterial (Variables|Default|Getshield) 0 (Variables|Default|GetM_shield)))